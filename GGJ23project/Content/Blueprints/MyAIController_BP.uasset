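; AI controller Blueprint that drives an agent through a behavior tree and feeds it perception results through a blackboard.
; BeginPlay starts the BehaviorTree logic.
; Perception updates involving a BP_Character print its name and store it as a blackboard object, without checking whether it was sensed or lost.
; Tick writes false to the PlayerHas blackboard flag every frame, and nothing here sets it true.
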(event OnTargetPerceptionUpdated(AIPerception)
  (params (Actor :type Actor%20Object%20Reference) (Stimulus :type AI%20Stimulus%20Structure))
  (bind _asbp_character (Utilities|Casting|CastToBP_Character Actor))
  (Development|PrintString (Utilities|GetDisplayName _asbp_character))
  (AI|Components|Blackboard|SetValueasObject (Variables|Default|GetBlackboard1) (Variables|Default|GetKey%20Name) Actor))

(event EventBeginPlay
  (AI|Logic|StartLogic (Variables|Default|GetBehaviorTree)))

(event EventTick
  (params (DeltaSeconds :type Float%20%28single-precision%29))
  (AI|Components|Blackboard|SetValueasBool (Variables|Default|GetBlackboard1) (Variables|Default|GetPlayerHas) false))

(fn ConstructionScript)