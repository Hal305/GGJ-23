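; BP_Pickup is a base pickup actor that the player can collect by pressing interact while standing inside its box.
; Box overlap with BP_PlayerCharacter binds the Interacted event to the player's InteractButtonPressed dispatcher, caches the player and shows a prompt text; leaving unbinds it and hides the text.
; Interacted calls PICKEDUP with the cached player, an empty event that serves as a hook for specific pickup behavior.
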(event OnComponentBeginOverlap(Box)
  (params (OverlappedComponent :type Primitive%20Component%20Object%20Reference) (OtherActor :type Actor%20Object%20Reference) (OtherComp :type Primitive%20Component%20Object%20Reference) (OtherBodyIndex :type Integer) (bFromSweep :type Boolean) (SweepResult :type Hit%20Result%20Structure%20%28by%20ref%29))
  (bind _asbp_player_character (Utilities|Casting|CastToBP_PlayerCharacter OtherActor))
  (EventDispatchers|BindEventtoInteractButtonPressed _asbp_player_character (delegate Custom|Interacted))
  (Variables|Default|Setplayer _asbp_player_character)
  (Rendering|SetVisibility (Variables|Default|GetText) true false))

(event OnComponentEndOverlap(Box)
  (params (OverlappedComponent :type Primitive%20Component%20Object%20Reference) (OtherActor :type Actor%20Object%20Reference) (OtherComp :type Primitive%20Component%20Object%20Reference) (OtherBodyIndex :type Integer))
  (bind _asbp_player_character (Utilities|Casting|CastToBP_PlayerCharacter OtherActor))
  (EventDispatchers|UnbindEventfromInteractButtonPressed _asbp_player_character (delegate Custom|Interacted))
  (Variables|Default|Setplayer _asbp_player_character)
  (Rendering|SetVisibility (Variables|Default|GetText) false false))

(event Custom|PICKED%20UP
  (params (Player :type BP%20Player%20Character%20Object%20Reference)))

(event Custom|Interacted
  (CallFunction|PICKEDUP (Variables|Default|Getplayer)))

(event EventBeginPlay)

(event Collision|EventActorBeginOverlap
  (params (OtherActor :type Actor%20Object%20Reference)))

(event EventTick
  (params (DeltaSeconds :type Float%20%28single-precision%29)))

(fn ConstructionScript)