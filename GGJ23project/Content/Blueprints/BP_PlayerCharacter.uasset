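; Player character Blueprint for a raccoon drawn with Paper2D flipbooks, handling its animation and the pause menu.
; Each tick, it picks a walk or idle flipbook from the last movement input, using the front or back version according to FacingCam, which is not set here.
; The Pause input creates the pause widget, switches to UI-only input, pauses the game and shows the mouse cursor.
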(event EventBeginPlay)

(event Collision|EventActorBeginOverlap
  (params (OtherActor :type Actor%20Object%20Reference)))

(event EventTick
  (params (DeltaSeconds :type Float%20%28single-precision%29))
  (bind _paperflipbook (Variables|Default|GetPaperFlipbook))
  (bind _bfacingcam (Variables|Default|GetbFacingCam))
  (Math|Float|CompareFloat (Math|Vector|VectorLengthSquared (Pawn|Components|PawnMovement|GetLastInputVector (Variables|Character|GetCharacterMovement))) 0.0
    (:>
      (if _bfacingcam
        (Sprite|SetFlipbook _paperflipbook "/Game/Sprites/Animation/Raccoon/WalkToCam/Raccoon_Walk_FrontFB.Raccoon_Walk_FrontFB")
        (else
          (Sprite|SetFlipbook _paperflipbook "/Game/Sprites/Animation/Raccoon/WalkAway/Raccoon_Walk_Back_FB.Raccoon_Walk_Back_FB"))))
    (:==
      (if _bfacingcam
        (Sprite|SetFlipbook (Variables|Default|GetPaperFlipbook) "/Game/Sprites/Animation/Raccoon_Idle_Front_FB.Raccoon_Idle_Front_FB")
        (else
          (Sprite|SetFlipbook (Variables|Default|GetPaperFlipbook) "/Game/Sprites/Animation/Raccoon_Idle_Back_FB.Raccoon_Idle_Back_FB"))))))

(event Input|ActionEvents|InputActionPause
  (params (Key :type Key%20Structure :default "None"))
  (:Pressed
    (bind _returnvalue (UserInterface|CreateWidget "/Game/Widget/WBP_Pause.WBP_Pause_C"))
    (bind _output_get (Variables|Default|SetPauseWidget _returnvalue))
    (UserInterface|Viewport|AddtoViewport _output_get 0)
    (bind _asplayer_controller (Utilities|Casting|CastToPlayerController (Pawn|GetController)))
    (Input|SetInputModeUIOnly _asplayer_controller _output_get "DoNotLock")
    (Game|SetGamePaused true)
    (Variables|/Script/Engine.PlayerController|SetbShowMouseCursor _asplayer_controller true)))

(fn ConstructionScript)