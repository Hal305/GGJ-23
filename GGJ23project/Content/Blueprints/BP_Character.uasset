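; BP_Character is a raccoon character drawn with a Paper2D flipbook.
; Each Tick checks the squared length of the movement component's last input vector to choose between walk and idle animations.
; The FacingCam flag then selects the front or back variant of that flipbook; this graph reads the flag but never sets it.
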(event EventBeginPlay)

(event Collision|EventActorBeginOverlap
  (params (OtherActor :type Actor%20Object%20Reference)))

(event EventTick
  (params (DeltaSeconds :type Float%20%28single-precision%29))
  (bind _paperflipbook (Variables|Default|GetPaperFlipbook))
  (bind _bfacingcam (Variables|Default|GetbFacingCam))
  (Math|Float|CompareFloat (Math|Vector|VectorLengthSquared (Pawn|Components|PawnMovement|GetLastInputVector (Variables|Character|GetCharacterMovement))) 0.0
    (:>
      (if _bfacingcam
        (Sprite|SetFlipbook _paperflipbook "/Game/Sprites/Animation/Raccoon/WalkToCam/Raccoon_Walk_Front_FB.Raccoon_Walk_Front_FB")
        (else
          (Sprite|SetFlipbook _paperflipbook "/Game/Sprites/Animation/Raccoon/WalkAway/Raccoon_Walk_Back_FB.Raccoon_Walk_Back_FB"))))
    (:==
      (if _bfacingcam
        (Sprite|SetFlipbook (Variables|Default|GetPaperFlipbook) "/Game/Sprites/Animation/Raccoon_Idle_Front_FB.Raccoon_Idle_Front_FB")
        (else
          (Sprite|SetFlipbook (Variables|Default|GetPaperFlipbook) "/Game/Sprites/Animation/Raccoon_Idle_Back_FB.Raccoon_Idle_Back_FB"))))))

(fn ConstructionScript)